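; BP_Tunnel is an endless-runner tunnel segment with a rotating holed wall, enemies and pickups.
; RandomizeWall picks the wall mesh and roll, then randomly removes health, ammo and enemy components.
; Hit events damage or resupply BP_Player, absorb projectiles, score shot enemies, and blank used meshes.
; Trigger overlap spawns the next tunnel via TunnelSpawner and destroys this one; end overlap commits TempScore to Score and calls ChangeSpeed.
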(event OnComponentBeginOverlap(TriggerZone)
  (params (OverlappedComponent :type Primitive%20Component%20Object%20Reference) (OtherActor :type Actor%20Object%20Reference) (OtherComp :type Primitive%20Component%20Object%20Reference) (OtherBodyIndex :type Integer) (bFromSweep :type Boolean) (SweepResult :type Hit%20Result%20Structure%20%28by%20ref%29))
  (bind _asbp_player (Utilities|Casting|CastToBP_Player OtherActor))
  (Variables|/Game/InfiniteMatrix/Blueprints/BP_Player.BP_Player_C|SetTempScore _asbp_player (+ (Variables|/Game/InfiniteMatrix/Blueprints/BP_Player.BP_Player_C|GetTempScore _asbp_player) 1))
  (Default|SpawnTunnelatSpawnPoint (Variables|Default|GetTunnelSpawner))
  (Actor|DestroyActor))

(event OnComponentHit(WallMesh)
  (params (HitComponent :type Primitive%20Component%20Object%20Reference) (OtherActor :type Actor%20Object%20Reference) (OtherComp :type Primitive%20Component%20Object%20Reference) (NormalImpulse :type Vector :default "0, 0, 0") (Hit :type Hit%20Result%20Structure%20%28by%20ref%29))
  (bind _asbp_player (Utilities|Casting|CastToBP_Player OtherActor)
    (:then
      (Game|Damage|ApplyDamage _asbp_player 25.0 0 0)
      (if (== (Variables|/Game/InfiniteMatrix/Blueprints/BP_Player.BP_Player_C|GetHealth _asbp_player) 0.0)
        (Variables|/Game/InfiniteMatrix/Blueprints/BP_Player.BP_Player_C|SetIsDead _asbp_player true)
        (Default|DisplayRestart _asbp_player)
        (else
          (Components|StaticMesh|SetStaticMesh (Variables|Default|GetWallMesh) 0)
          (bind _asbp_player_2 (Utilities|Casting|CastToBP_Player (Game|Player|GetPlayerPawn 0)))
          (Variables|/Game/InfiniteMatrix/Blueprints/BP_Player.BP_Player_C|SetTempScore _asbp_player_2 (- (Variables|/Game/InfiniteMatrix/Blueprints/BP_Player.BP_Player_C|GetTempScore _asbp_player_2) 1)))))
    (:CastFailed
      (bind _asbp_projectile (Utilities|Casting|CastToBP_Projectile OtherActor))
      (Actor|DestroyActor _asbp_projectile))))

(event OnComponentHit(EnemyFive)
  (params (HitComponent :type Primitive%20Component%20Object%20Reference) (OtherActor :type Actor%20Object%20Reference) (OtherComp :type Primitive%20Component%20Object%20Reference) (NormalImpulse :type Vector :default "0, 0, 0") (Hit :type Hit%20Result%20Structure%20%28by%20ref%29))
  (bind _asbp_player (Utilities|Casting|CastToBP_Player OtherActor)
    (:then
      (Components|StaticMesh|SetStaticMesh (Variables|Default|GetEnemyFive) 0)
      (Game|Damage|ApplyDamage _asbp_player 25.0 0 0)
      (if (== (Variables|/Game/InfiniteMatrix/Blueprints/BP_Player.BP_Player_C|GetHealth _asbp_player) 0.0)
        (Variables|/Game/InfiniteMatrix/Blueprints/BP_Player.BP_Player_C|SetIsDead _asbp_player true)
        (Default|DisplayRestart _asbp_player)))
    (:CastFailed
      (bind _asbp_projectile (Utilities|Casting|CastToBP_Projectile OtherActor))
      (Actor|DestroyActor _asbp_projectile)
      (Components|StaticMesh|SetStaticMesh (Variables|Default|GetEnemyFive) 0)
      (bind _asbp_player_2 (Utilities|Casting|CastToBP_Player (Game|Player|GetPlayerPawn 0)))
      (Variables|/Game/InfiniteMatrix/Blueprints/BP_Player.BP_Player_C|SetScore _asbp_player_2 (+ (Variables|/Game/InfiniteMatrix/Blueprints/BP_Player.BP_Player_C|GetScore _asbp_player_2) 1))
      (Variables|/Game/InfiniteMatrix/Blueprints/BP_Player.BP_Player_C|SetTempScore _asbp_player_2 (+ (Variables|/Game/InfiniteMatrix/Blueprints/BP_Player.BP_Player_C|GetTempScore _asbp_player_2) 1)))))

(event OnComponentHit(AmmoOne)
  (params (HitComponent :type Primitive%20Component%20Object%20Reference) (OtherActor :type Actor%20Object%20Reference) (OtherComp :type Primitive%20Component%20Object%20Reference) (NormalImpulse :type Vector :default "0, 0, 0") (Hit :type Hit%20Result%20Structure%20%28by%20ref%29))
  (bind _asbp_player (Utilities|Casting|CastToBP_Player OtherActor)
    (:then
      (Variables|/Game/InfiniteMatrix/Blueprints/BP_Player.BP_Player_C|SetAmmo _asbp_player (Math|Integer|Clamp(Integer) (+ (Variables|/Game/InfiniteMatrix/Blueprints/BP_Player.BP_Player_C|GetAmmo _asbp_player) 10) 0 75))
      (Components|StaticMesh|SetStaticMesh (Variables|Default|GetAmmoOne) 0))
    (:CastFailed
      (bind _asbp_projectile (Utilities|Casting|CastToBP_Projectile OtherActor))
      (Actor|DestroyActor _asbp_projectile))))

(event OnComponentHit(AmmoTwo)
  (params (HitComponent :type Primitive%20Component%20Object%20Reference) (OtherActor :type Actor%20Object%20Reference) (OtherComp :type Primitive%20Component%20Object%20Reference) (NormalImpulse :type Vector :default "0, 0, 0") (Hit :type Hit%20Result%20Structure%20%28by%20ref%29))
  (bind _asbp_player (Utilities|Casting|CastToBP_Player OtherActor)
    (:then
      (Variables|/Game/InfiniteMatrix/Blueprints/BP_Player.BP_Player_C|SetAmmo _asbp_player (Math|Integer|Clamp(Integer) (+ (Variables|/Game/InfiniteMatrix/Blueprints/BP_Player.BP_Player_C|GetAmmo _asbp_player) 10) 0 75))
      (Components|StaticMesh|SetStaticMesh (Variables|Default|GetAmmoTwo) 0))
    (:CastFailed
      (bind _asbp_projectile (Utilities|Casting|CastToBP_Projectile OtherActor))
      (Actor|DestroyActor _asbp_projectile))))

(event OnComponentEndOverlap(TriggerZone)
  (params (OverlappedComponent :type Primitive%20Component%20Object%20Reference) (OtherActor :type Actor%20Object%20Reference) (OtherComp :type Primitive%20Component%20Object%20Reference) (OtherBodyIndex :type Integer))
  (bind _asbp_player (Utilities|Casting|CastToBP_Player OtherActor))
  (Variables|/Game/InfiniteMatrix/Blueprints/BP_Player.BP_Player_C|SetScore _asbp_player (Variables|/Game/InfiniteMatrix/Blueprints/BP_Player.BP_Player_C|GetTempScore _asbp_player))
  (Default|ChangeSpeed _asbp_player)
  (if (Variables|Default|GetHealthPackValid)
    (Components|DestroyComponent (Variables|Default|GetHealthPack)))
  (if (Variables|Default|GetEnOne)
    (Components|DestroyComponent (Variables|Default|GetEnemyOne)))
  (if (Variables|Default|GetEnTwo)
    (Components|DestroyComponent (Variables|Default|GetEmemyTwo)))
  (if (Variables|Default|GetEnThree)
    (Components|DestroyComponent (Variables|Default|GetEnemyThree)))
  (if (Variables|Default|GetEnFour)
    (Components|DestroyComponent (Variables|Default|GetEnemyFour)))
  (if (Variables|Default|GetEnFive)
    (Components|DestroyComponent (Variables|Default|GetEnemyFive)))
  (if (Variables|Default|GetAmOne)
    (Components|DestroyComponent (Variables|Default|GetAmmoOne)))
  (if (Variables|Default|GetAmTwo)
    (Components|DestroyComponent (Variables|Default|GetAmmoTwo))))

(event OnComponentHit(HealthPack)
  (params (HitComponent :type Primitive%20Component%20Object%20Reference) (OtherActor :type Actor%20Object%20Reference) (OtherComp :type Primitive%20Component%20Object%20Reference) (NormalImpulse :type Vector :default "0, 0, 0") (Hit :type Hit%20Result%20Structure%20%28by%20ref%29))
  (bind _asbp_player (Utilities|Casting|CastToBP_Player OtherActor)
    (:then
      (Variables|/Game/InfiniteMatrix/Blueprints/BP_Player.BP_Player_C|SetHealth _asbp_player (Math|Float|Clamp(Float) (+ (Variables|/Game/InfiniteMatrix/Blueprints/BP_Player.BP_Player_C|GetHealth _asbp_player) 25.0) 0.0 1e+02))
      (Components|StaticMesh|SetStaticMesh (Variables|Default|GetHealthPack) 0))
    (:CastFailed
      (bind _asbp_projectile (Utilities|Casting|CastToBP_Projectile OtherActor))
      (Actor|DestroyActor _asbp_projectile))))

(event OnComponentHit(StaticMeshComponent)
  (params (HitComponent :type Primitive%20Component%20Object%20Reference) (OtherActor :type Actor%20Object%20Reference) (OtherComp :type Primitive%20Component%20Object%20Reference) (NormalImpulse :type Vector :default "0, 0, 0") (Hit :type Hit%20Result%20Structure%20%28by%20ref%29))
  (bind _asbp_projectile (Utilities|Casting|CastToBP_Projectile OtherActor))
  (Actor|DestroyActor _asbp_projectile))

(event OnComponentHit(EnemyOne)
  (params (HitComponent :type Primitive%20Component%20Object%20Reference) (OtherActor :type Actor%20Object%20Reference) (OtherComp :type Primitive%20Component%20Object%20Reference) (NormalImpulse :type Vector :default "0, 0, 0") (Hit :type Hit%20Result%20Structure%20%28by%20ref%29))
  (bind _asbp_player (Utilities|Casting|CastToBP_Player OtherActor)
    (:then
      (Components|StaticMesh|SetStaticMesh (Variables|Default|GetEnemyOne) 0)
      (Game|Damage|ApplyDamage _asbp_player 25.0 0 0)
      (if (== (Variables|/Game/InfiniteMatrix/Blueprints/BP_Player.BP_Player_C|GetHealth _asbp_player) 0.0)
        (Variables|/Game/InfiniteMatrix/Blueprints/BP_Player.BP_Player_C|SetIsDead _asbp_player true)
        (Default|DisplayRestart _asbp_player)))
    (:CastFailed
      (bind _asbp_projectile (Utilities|Casting|CastToBP_Projectile OtherActor))
      (Actor|DestroyActor _asbp_projectile)
      (Components|StaticMesh|SetStaticMesh (Variables|Default|GetEnemyOne) 0)
      (bind _asbp_player_2 (Utilities|Casting|CastToBP_Player (Game|Player|GetPlayerPawn 0)))
      (Variables|/Game/InfiniteMatrix/Blueprints/BP_Player.BP_Player_C|SetScore _asbp_player_2 (+ (Variables|/Game/InfiniteMatrix/Blueprints/BP_Player.BP_Player_C|GetScore _asbp_player_2) 1))
      (Variables|/Game/InfiniteMatrix/Blueprints/BP_Player.BP_Player_C|SetTempScore _asbp_player_2 (+ (Variables|/Game/InfiniteMatrix/Blueprints/BP_Player.BP_Player_C|GetTempScore _asbp_player_2) 1)))))

(event OnComponentHit(EmemyTwo)
  (params (HitComponent :type Primitive%20Component%20Object%20Reference) (OtherActor :type Actor%20Object%20Reference) (OtherComp :type Primitive%20Component%20Object%20Reference) (NormalImpulse :type Vector :default "0, 0, 0") (Hit :type Hit%20Result%20Structure%20%28by%20ref%29))
  (bind _asbp_player (Utilities|Casting|CastToBP_Player OtherActor)
    (:then
      (Components|StaticMesh|SetStaticMesh (Variables|Default|GetEmemyTwo) 0)
      (Game|Damage|ApplyDamage _asbp_player 25.0 0 0)
      (if (== (Variables|/Game/InfiniteMatrix/Blueprints/BP_Player.BP_Player_C|GetHealth _asbp_player) 0.0)
        (Variables|/Game/InfiniteMatrix/Blueprints/BP_Player.BP_Player_C|SetIsDead _asbp_player true)
        (Default|DisplayRestart _asbp_player)))
    (:CastFailed
      (bind _asbp_projectile (Utilities|Casting|CastToBP_Projectile OtherActor))
      (Actor|DestroyActor _asbp_projectile)
      (Components|StaticMesh|SetStaticMesh (Variables|Default|GetEmemyTwo) 0)
      (bind _asbp_player_2 (Utilities|Casting|CastToBP_Player (Game|Player|GetPlayerPawn 0)))
      (Variables|/Game/InfiniteMatrix/Blueprints/BP_Player.BP_Player_C|SetScore _asbp_player_2 (+ (Variables|/Game/InfiniteMatrix/Blueprints/BP_Player.BP_Player_C|GetScore _asbp_player_2) 1))
      (Variables|/Game/InfiniteMatrix/Blueprints/BP_Player.BP_Player_C|SetTempScore _asbp_player_2 (+ (Variables|/Game/InfiniteMatrix/Blueprints/BP_Player.BP_Player_C|GetTempScore _asbp_player_2) 1)))))

(event OnComponentHit(EnemyThree)
  (params (HitComponent :type Primitive%20Component%20Object%20Reference) (OtherActor :type Actor%20Object%20Reference) (OtherComp :type Primitive%20Component%20Object%20Reference) (NormalImpulse :type Vector :default "0, 0, 0") (Hit :type Hit%20Result%20Structure%20%28by%20ref%29))
  (bind _asbp_player (Utilities|Casting|CastToBP_Player OtherActor)
    (:then
      (Components|StaticMesh|SetStaticMesh (Variables|Default|GetEnemyThree) 0)
      (Game|Damage|ApplyDamage _asbp_player 25.0 0 0)
      (if (== (Variables|/Game/InfiniteMatrix/Blueprints/BP_Player.BP_Player_C|GetHealth _asbp_player) 0.0)
        (Variables|/Game/InfiniteMatrix/Blueprints/BP_Player.BP_Player_C|SetIsDead _asbp_player true)
        (Default|DisplayRestart _asbp_player)))
    (:CastFailed
      (bind _asbp_projectile (Utilities|Casting|CastToBP_Projectile OtherActor))
      (Actor|DestroyActor _asbp_projectile)
      (Components|StaticMesh|SetStaticMesh (Variables|Default|GetEnemyThree) 0)
      (bind _asbp_player_2 (Utilities|Casting|CastToBP_Player (Game|Player|GetPlayerPawn 0)))
      (Variables|/Game/InfiniteMatrix/Blueprints/BP_Player.BP_Player_C|SetScore _asbp_player_2 (+ (Variables|/Game/InfiniteMatrix/Blueprints/BP_Player.BP_Player_C|GetScore _asbp_player_2) 1))
      (Variables|/Game/InfiniteMatrix/Blueprints/BP_Player.BP_Player_C|SetTempScore _asbp_player_2 (+ (Variables|/Game/InfiniteMatrix/Blueprints/BP_Player.BP_Player_C|GetTempScore _asbp_player_2) 1)))))

(event OnComponentHit(EnemyFour)
  (params (HitComponent :type Primitive%20Component%20Object%20Reference) (OtherActor :type Actor%20Object%20Reference) (OtherComp :type Primitive%20Component%20Object%20Reference) (NormalImpulse :type Vector :default "0, 0, 0") (Hit :type Hit%20Result%20Structure%20%28by%20ref%29))
  (bind _asbp_player (Utilities|Casting|CastToBP_Player OtherActor)
    (:then
      (Components|StaticMesh|SetStaticMesh (Variables|Default|GetEnemyFour) 0)
      (Game|Damage|ApplyDamage _asbp_player 25.0 0 0)
      (if (== (Variables|/Game/InfiniteMatrix/Blueprints/BP_Player.BP_Player_C|GetHealth _asbp_player) 0.0)
        (Variables|/Game/InfiniteMatrix/Blueprints/BP_Player.BP_Player_C|SetIsDead _asbp_player true)
        (Default|DisplayRestart _asbp_player)))
    (:CastFailed
      (bind _asbp_projectile (Utilities|Casting|CastToBP_Projectile OtherActor))
      (Actor|DestroyActor _asbp_projectile)
      (Components|StaticMesh|SetStaticMesh (Variables|Default|GetEnemyFour) 0)
      (bind _asbp_player_2 (Utilities|Casting|CastToBP_Player (Game|Player|GetPlayerPawn 0)))
      (Variables|/Game/InfiniteMatrix/Blueprints/BP_Player.BP_Player_C|SetScore _asbp_player_2 (+ (Variables|/Game/InfiniteMatrix/Blueprints/BP_Player.BP_Player_C|GetScore _asbp_player_2) 1))
      (Variables|/Game/InfiniteMatrix/Blueprints/BP_Player.BP_Player_C|SetTempScore _asbp_player_2 (+ (Variables|/Game/InfiniteMatrix/Blueprints/BP_Player.BP_Player_C|GetTempScore _asbp_player_2) 1)))))

(event EventTick
  (params (DeltaSeconds :type Float%20%28single-precision%29))
  (Transformation|AddLocalRotation (Variables|Default|GetWallMesh) (Math|Rotator|MakeRotator (* DeltaSeconds (Variables|Default|GetRotateSpeed)) 0.0 0.0) false false))

(fn ConstructionScript)

(fn RandomizeWall
  (bind _returnvalue (Math|Random|RandomIntegerinRange 0 6))
  (bind _returnvalue_2 (> _returnvalue 0))
  (Utilities|FlowControl|Sequence
    (:then_0
      (Components|StaticMesh|SetStaticMesh (Variables|Default|GetWallMesh) (Utilities|Select :Index (Math|Random|RandomIntegerinRange 0 3) :Option%200 "/Game/InfiniteMatrix/Meshes/SM_Hole_01.SM_Hole_01" :Option%201 "/Game/InfiniteMatrix/Meshes/SM_Hole_02.SM_Hole_02" :Option%202 "/Game/InfiniteMatrix/Meshes/SM_Hole_03.SM_Hole_03" :Option%203 "/Game/InfiniteMatrix/Meshes/SM_Hole_04.SM_Hole_04"))
      (Transformation|AddLocalRotation (Variables|Default|GetWallMesh) (Math|Rotator|MakeRotator (Math|Random|RandomFloatinRange 0.0 3.6e+02) 0.0 0.0) false false))
    (:then_1
      (Utilities|FlowControl|Sequence
        (:then_0
          (if (== (Math|Random|RandomIntegerinRange 0 5) 0)
            (Variables|Default|SetHealthPackValid true)
            (else
              (Components|DestroyComponent (Variables|Default|GetHealthPack))
              (Variables|Default|SetHealthPackValid false))))
        (:then_1
          (Utilities|FlowControl|Sequence
            (:then_0
              (if (> (Math|Random|RandomIntegerinRange 0 5) 0)
                (Components|DestroyComponent (Variables|Default|GetEnemyOne))
                (Variables|Default|SetEnOne false)
                (if (> (Math|Random|RandomIntegerinRange 0 5) 0)
                  (Components|DestroyComponent (Variables|Default|GetEmemyTwo))
                  (Variables|Default|SetEnTwo false)
                  (if (> (Math|Random|RandomIntegerinRange 0 5) 0)
                    (Components|DestroyComponent (Variables|Default|GetEnemyThree))
                    (Variables|Default|SetEnThree false)
                    (if (> (Math|Random|RandomIntegerinRange 0 5) 0)
                      (Components|DestroyComponent (Variables|Default|GetEnemyFour))
                      (Variables|Default|SetEnFour false)
                      (if (> (Math|Random|RandomIntegerinRange 0 5) 0)
                        (Components|DestroyComponent (Variables|Default|GetEnemyFive))
                        (Variables|Default|SetEnFive false)))))))
            (:then_1
              (if (== (Math|Random|RandomIntegerinRange 0 1) 0)
                (Components|DestroyComponent (Variables|Default|GetAmmoOne))
                (Variables|Default|SetAmOne false)
                (if _returnvalue_2
                  (Components|DestroyComponent (Variables|Default|GetAmmoTwo))
                  (Variables|Default|SetAmTwo false))
                (else
                  (Components|DestroyComponent (Variables|Default|GetAmmoTwo))
                  (Variables|Default|SetAmTwo false)
                  (if _returnvalue_2
                    (Components|DestroyComponent (Variables|Default|GetAmmoOne))
                    (Variables|Default|SetAmOne false)))))))))))